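; Combat library whose Attack function picks an attack branch for player 0's BP_CoopCharacter from its stun, dodge-window and dodge-combo-window flags.
; Stun feedback and the attack and special-attack flipbooks are only commented placeholders with no logic wired.
; Outside those three states, it sets AttackComboWindow true when the current playback frame lies within the inclusive ComboWindowFirst–ComboWindowLast range, and false otherwise.
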(fn `Attack`
  (params (ComboWindowFirst :type Integer) (ComboWindowLast :type Integer))
  (bind _returnvalue (`PaperFlipbookComponent.GetPlaybackPositionInFrames`))
  (bind _asbp_coop_character (cast `/Game/Assets/Characters/BaseCharacter/Blueprints/Character/BP_CoopCharacter` (`GameplayStatics.GetPlayerCharacter` null)))
  (if (`/Game/Assets/Characters/BaseCharacter/Blueprints/Character/BP_CoopCharacter.IsCharStunned?` _asbp_coop_character)
    ;[1 1 1] feedback visual
    (`|ExecutionSequence`)
    (elif (`/Game/Assets/Characters/BaseCharacter/Blueprints/Character/BP_CoopCharacter.DodgeWindow` _asbp_coop_character)
      ;[1 1 1] play flip book attack 2
      (`|ExecutionSequence`)
      (else
        ;[1 1 1] play flip book attack 1
        (`|ExecutionSequence`
          (:`then_0`
            (if (`/Game/Assets/Characters/BaseCharacter/Blueprints/Character/BP_CoopCharacter.DodgeComboWindow` _asbp_coop_character)
              ;[1 1 1] play flip book specialattack
              (`|ExecutionSequence`)
              (else
                (`/Engine/EditorBlueprintResources/StandardMacros.CompareInt` _returnvalue ComboWindowFirst
                  (:`>`
                    (`/Engine/EditorBlueprintResources/StandardMacros.CompareInt` _returnvalue ComboWindowLast :!label _label
                      (:`>`
                        (set `/Game/Assets/Characters/BaseCharacter/Blueprints/Character/BP_CoopCharacter.AttackComboWindow` false _asbp_coop_character :!label _label_2))
                      (:`==`
                        (set `/Game/Assets/Characters/BaseCharacter/Blueprints/Character/BP_CoopCharacter.AttackComboWindow` true _asbp_coop_character :!label _label_3))
                      (:`<`
                        (goto _label_3))))
                  (:`==`
                    (goto _label))
                  (:`<`
                    (goto _label_2)))))))))))